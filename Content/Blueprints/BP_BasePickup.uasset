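; Base pickup actor that the third-person character collects as candy.
; On BeginPlay, after a brief delay, the TimelineChange and Random flags select one of three timelines that animate the Sphere's relative location.
; When BP_ThirdPersonCharacter overlaps the Sphere, it increments that character's NumCandy, passes the result to CallScoreCandy and destroys itself.
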(event `self.ReceiveBeginPlay`
  (`KismetSystemLibrary.Delay` 0.02)
  (if (`self.TimelineChange`)
    (if (`self.Random`)
      (bind (_direction _x _y _z) (`Timeline|Timeline_1`)
        (:`Update`
          (`SceneComponent.K2_SetRelativeLocation` (`self.Sphere`) (`KismetMathLibrary.MakeVector` _x _y _z) false false)))
      (else
        (bind (_direction_2 _x_2 _y_2 _z_2) (`Timeline|Timeline`)
          (:`Update`
            (`SceneComponent.K2_SetRelativeLocation` (`self.Sphere`) (`KismetMathLibrary.MakeVector` _x_2 _y_2 _z_2) false false)))))
    (else
      (bind (_direction_3 _x_3 _y_3 _z_3) (`Timeline|Timeline_2`)
        (:`Update`
          (`SceneComponent.K2_SetRelativeLocation` (`self.Sphere`) (`KismetMathLibrary.MakeVector` _x_3 _y_3 _z_3) false false))))))

(event `self.Sphere.OnComponentBeginOverlap`
  (params (OverlappedComponent :type "PrimitiveComponent Object Reference") (OtherActor :type "Actor Object Reference") (OtherComp :type "PrimitiveComponent Object Reference") (OtherBodyIndex :type Integer) (bFromSweep :type Boolean) (SweepResult :type "HitResult Structure (by ref)"))
  (bind _asbp_third_person_character (cast `/Game/ThirdPerson/Blueprints/BP_ThirdPersonCharacter` OtherActor))
  (bind _result (`/Engine/EditorBlueprintResources/StandardMacros.IncrementInt` (`/Game/ThirdPerson/Blueprints/BP_ThirdPersonCharacter.Num Candy` _asbp_third_person_character))
    (:`  `
      (`self.ScoreCandy` _result)
      (`self.K2_DestroyActor`))))

(fn `UserConstructionScript`)