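; BP_Goblin is a goblin actor that plays an aggro animation shortly after BeginPlay, then spawns pickups at its own location.
; A delayed loop spawns a BP_BasePickup from the Class array at each CountDown index until the counter reaches three.
; Nested FlipFlops alternate each pickup's TimelineChange flag and, when that is true, its Random flag, so successive pickups are configured differently.
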(event `self.ReceiveBeginPlay`
  (`KismetSystemLibrary.Delay` 0.5)
  (`SkeletalMeshComponent.PlayAnimation` (`self.Mesh`) "/Game/UndeadPack/EnemyGoblin/Animations/Anim_Agr.Anim_Agr" false)
  (`KismetSystemLibrary.Delay` 0.5)
  (if (not (== (`self.CountDown`) 3)) :!label _label
    (bind _returnvalue (`|SpawnActorFromClass` (`|GetArrayItem` (`self.Class`) (`self.CountDown`)) (`KismetMathLibrary.MakeTransform` (`self.K2_GetActorLocation`) (`self.K2_GetActorRotation`)) "Undefined" "MultiplyWithRoot" null null))
    (bind _asbp_base_pickup (cast `/Game/Blueprints/BP_BasePickup` _returnvalue))
    (set `self.BasePickup` _asbp_base_pickup)
    (`/Engine/EditorBlueprintResources/StandardMacros.FlipFlop`
      (:`A`
        (set `/Game/Blueprints/BP_BasePickup.TimelineChange` true (`self.BasePickup`))
        (`/Engine/EditorBlueprintResources/StandardMacros.FlipFlop`
          (:`A`
            (set `/Game/Blueprints/BP_BasePickup.Random` true (`self.BasePickup`)))
          (:`B`
            (set `/Game/Blueprints/BP_BasePickup.Random` false (`self.BasePickup`)))))
      (:`B`
        (set `/Game/Blueprints/BP_BasePickup.TimelineChange` false (`self.BasePickup`))))
    (`/Engine/EditorBlueprintResources/StandardMacros.IncrementInt` (`self.CountDown`)
      (:`  `
        (`KismetSystemLibrary.Delay` 0.02)
        (goto _label)))))

(fn `UserConstructionScript`)