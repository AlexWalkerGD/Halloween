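; BP_Lich is a Lich hazard that kills the third-person player when they enter its sphere trigger.
; On overlap it flags the player Dead, plays a spell animation, and shows the game over widget after a short delay.
; It also zeroes the player's walk speed while a timeline drives the player mesh's relative Z.
; The construction script sets the template on its smoke and particle components.
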(event `self.Sphere.OnComponentBeginOverlap`
  (params (OverlappedComponent :type "PrimitiveComponent Object Reference") (OtherActor :type "Actor Object Reference") (OtherComp :type "PrimitiveComponent Object Reference") (OtherBodyIndex :type Integer) (bFromSweep :type Boolean) (SweepResult :type "HitResult Structure (by ref)"))
  (bind _asbp_third_person_character (cast `/Game/ThirdPerson/Blueprints/BP_ThirdPersonCharacter` OtherActor))
  (`|ExecutionSequence`
    (:`then_0`
      (set `/Game/ThirdPerson/Blueprints/BP_ThirdPersonCharacter.Dead` true _asbp_third_person_character)
      (`SkeletalMeshComponent.PlayAnimation` (`self.Mesh`) "/Game/UndeadPack/Lich/Animations/Anim_Spell.Anim_Spell" false)
      (`KismetSystemLibrary.Delay` 2.0)
      (bind _returnvalue (`|CreateWidget` "/Game/UI/W_GameOver.W_GameOver_C"))
      (`UserWidget.AddToViewport` _returnvalue 0))
    (:`then_1`
      (set `CharacterMovementComponent.MaxWalkSpeed` 0.0 (`Character.CharacterMovement` _asbp_third_person_character))
      (bind (_direction _newtrack_0) (`Timeline|Timeline`)
        (:`Update`
          (bind _mesh (`Character.Mesh` _asbp_third_person_character))
          (bind (_relativelocation_x _relativelocation_y) (`KismetMathLibrary.BreakVector` (`SceneComponent.RelativeLocation` _mesh)))
          (`SceneComponent.K2_SetRelativeLocation` _mesh (`KismetMathLibrary.MakeVector` _relativelocation_x _relativelocation_y _newtrack_0) false false))))))

(fn `UserConstructionScript`
  (`ParticleSystemComponent.SetTemplate` (`self.Smoke_FX`) (`self.Template`))
  (`ParticleSystemComponent.SetTemplate` (`self.ParticleSystem`) (`self.Template`)))